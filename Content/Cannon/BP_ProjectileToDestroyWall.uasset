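; Cannon projectile that breaks a BP_Wall on impact and hands player control to a newly spawned BP_Cherry.
; A hit on the Sphere component tells the wall to destroy itself, then after a short delay spawns the cherry at the projectile's location.
; Once that spawn is valid, player controller 0 possesses it, the Cannon hides its path and resets firing, and the projectile destroys itself.
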(event `self.Sphere.OnComponentHit`
  (params (HitComponent :type "PrimitiveComponent Object Reference") (OtherActor :type "Actor Object Reference") (OtherComp :type "PrimitiveComponent Object Reference") (NormalImpulse :type "Vector Structure") (Hit :type "HitResult Structure (by ref)"))
  (bind _returnvalue_location (`KismetMathLibrary.BreakTransform` (`self.GetTransform`)))
  (bind _cannon (`self.Cannon`))
  (bind _asbp_wall (cast `/Game/Cannon/BP_Wall` OtherActor))
  (`/Game/Cannon/BP_Wall.Destroy Wall` _asbp_wall)
  (`KismetSystemLibrary.Delay` 0.4)
  (bind _returnvalue (`|SpawnActorFromClass` "/Game/Characters/BP_Cherry.BP_Cherry_C" (`KismetMathLibrary.MakeTransform` _returnvalue_location) "Undefined" "MultiplyWithRoot" null null))
  (`/Engine/EditorBlueprintResources/StandardMacros.IsValid` _returnvalue
    (:`Is Valid`
      (`Controller.Possess` (`GameplayStatics.GetPlayerController` 0) _returnvalue)
      (`/Game/Cannon/BP_CannonToTravel.Hide Path` _cannon)
      (`/Game/Cannon/BP_CannonToTravel.Reset Fire` _cannon)
      (`self.K2_DestroyActor`))))

(fn `UserConstructionScript`
  (`parent.UserConstructionScript`))