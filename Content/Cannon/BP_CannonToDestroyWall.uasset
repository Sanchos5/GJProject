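; Cannon Blueprint that fires a BP_ProjectileToDestroyWall when the IA_Fire input starts.
; It spawns the projectile at the SpawnFruit transform, passes itself as the Cannon reference, sets the velocity from MissleVelocity and plays a 2D cannon sound.
; A DoOnce gate blocks further shots until CustomEvent resets it.
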(event `EnhancedInput|/Game/Input/Actions/IA_Fire`
  (params (ActionValue :type Boolean) (ElapsedSeconds :type "Float (double-precision)") (TriggeredSeconds :type "Float (double-precision)") (InputAction :type "InputAction Object Reference" :default "/Game/Input/Actions/IA_Fire.IA_Fire"))
  (bind (_returnvalue_location _returnvalue_rotation) (`KismetMathLibrary.BreakTransform` (`SceneComponent.K2_GetComponentToWorld` (`self.SpawnFruit`))))
  (:`Started`
    (`/Engine/EditorBlueprintResources/StandardMacros.DoOnce` false :!label _label
      (:`Completed`
        (bind _returnvalue (`|SpawnActorFromClass` "/Game/Cannon/BP_ProjectileToDestroyWall.BP_ProjectileToDestroyWall_C" (`KismetMathLibrary.MakeTransform` _returnvalue_location _returnvalue_rotation) "AlwaysSpawn" "MultiplyWithRoot" null self null))
        (set `MovementComponent.Velocity` (`self.Missle Velocity`) (`/Game/Cannon/BP_ProjectileToTravel.ProjectileMovement` _returnvalue))
        (`GameplayStatics.PlaySound2D` "/Game/Sound/S_CanonLong.S_CanonLong" 1.0 1.0 0.0 null null)))))

(event `CustomEvent`
  (goto _label :!via `Reset`))

(fn `UserConstructionScript`
  (`parent.UserConstructionScript`))