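; BP_Orange is an orange fruit character that splits off copies of itself and reacts to touching other fruit.
; Pressing E plays a sound and spawns another orange ahead, tracked in an array up to a slice limit.
; Overlapping a tracked copy removes it; a non-player cherry or dragon fruit sets a fruit number on BP_Controller, fires its event and destroys this orange.
; The final non-player orange branch is unreachable behind the first orange cast.
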(event `Key|E`
  (params (Key :type "Key Structure"))
  (:`Pressed`
    (`self.Division Into Lobules`)
    (`GameplayStatics.PlaySound2D` "/Game/Sound/S_OrangeDevide2.S_OrangeDevide2" 1.0 1.0 0.0 null null)))

(event `self.CapsuleComponent.OnComponentBeginOverlap`
  (params (OverlappedComponent :type "PrimitiveComponent Object Reference") (OtherActor :type "Actor Object Reference") (OtherComp :type "PrimitiveComponent Object Reference") (OtherBodyIndex :type Integer) (bFromSweep :type Boolean) (SweepResult :type "HitResult Structure (by ref)"))
  (bind _array (`self.Array`))
  (bind _asbp_orange (cast `/Game/Characters/BP_Orange` OtherActor)
    (:`then`
      (bind _returnvalue (`KismetArrayLibrary.Array_Find` _array _asbp_orange))
      (bind _output (`|GetArrayItem` _array _returnvalue))
      (`/Engine/EditorBlueprintResources/StandardMacros.IsValid` _output
        (:`Is Valid`
          (`self.K2_DestroyActor` _output)
          (`KismetArrayLibrary.Array_Remove` _array _returnvalue))))
    (:`CastFailed`
      (bind _asbp_cherry (cast `/Game/Characters/BP_Cherry` OtherActor)
        (:`then`
          (if (not (`/Game/Characters/BP_Cherry.player?` _asbp_cherry))
            (bind _asbp_controller (cast `/Game/Characters/BP_Controller` (`GameplayStatics.GetPlayerController` 0)))
            (set `/Game/Characters/BP_Controller.i_skolko_fruktov` 2 _asbp_controller)
            (`/Game/Characters/BP_Controller.Event_skolko_fructov` _asbp_controller)
            (`self.K2_DestroyActor` :!label _label)))
        (:`CastFailed`
          (bind _asbp_dragon_fruit (cast `/Game/Characters/BP_DragonFruit` OtherActor)
            (:`then`
              (if (not (`/Game/Characters/BP_DragonFruit.player?` _asbp_dragon_fruit))
                (bind _asbp_controller_2 (cast `/Game/Characters/BP_Controller` (`GameplayStatics.GetPlayerController` 0)))
                (set `/Game/Characters/BP_Controller.i_skolko_fruktov` 3 _asbp_controller_2)
                (`/Game/Characters/BP_Controller.Event_skolko_fructov` _asbp_controller_2)
                (goto _label)))
            (:`CastFailed`
              (bind _asbp_orange_2 (cast `/Game/Characters/BP_Orange` OtherActor))
              (if (not (`/Game/Characters/BP_Orange.player?` _asbp_orange_2))
                (bind _asbp_controller_3 (cast `/Game/Characters/BP_Controller` (`GameplayStatics.GetPlayerController` 0)))
                (set `/Game/Characters/BP_Controller.i_skolko_fruktov` 4 _asbp_controller_3)
                (`/Game/Characters/BP_Controller.Event_skolko_fructov` _asbp_controller_3)
                (goto _label)))))))))

(fn `Division Into Lobules`
  (if (not (>= (`KismetArrayLibrary.Array_Length` (`self.Array`)) (`self.Number of slices`)))
    (bind _returnvalue (`|SpawnActorFromClass` "BP_Orange_C" (`KismetMathLibrary.MakeTransform` (+ (* (`self.GetActorForwardVector` self) 150.0) (.location (`self.GetTransform` self))) (.rotation (`self.GetTransform` self)) (.scale (`self.GetTransform` self))) "AdjustIfPossibleButAlwaysSpawn" "MultiplyWithRoot" null null))
    (`KismetArrayLibrary.Array_Add` (`self.Array`) _returnvalue)))

(fn `UserConstructionScript`)