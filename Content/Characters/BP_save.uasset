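; Checkpoint trigger actor that saves the player's position when the player character enters its box volume.
; On BeginPlay it caches the custom game instance reference.
; A BasePlayerCharacter overlap writes that character's transform into the game instance's LocalSave and raises the SaveActive flag.
; It then calls EventSave on the first player's BP_Controller, which handles the rest of the save outside this asset.
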(event `self.ReceiveBeginPlay`
  (bind _asmy_game_instanse (cast `/Game/Characters/My_GameInstanse` (`GameplayStatics.GetGameInstance`)))
  (set `self.As My Game Instanse` _asmy_game_instanse))

(event `self.Box.OnComponentBeginOverlap`
  (params (OverlappedComponent :type "PrimitiveComponent Object Reference") (OtherActor :type "Actor Object Reference") (OtherComp :type "PrimitiveComponent Object Reference") (OtherBodyIndex :type Integer) (bFromSweep :type Boolean) (SweepResult :type "HitResult Structure (by ref)"))
  (bind _as_my_game_instanse (`self.As My Game Instanse`))
  ;[1 1 1] Если игрок зашёл в зону, запиши информацию о нём в гейм инстансе
  (bind _asbase_player_character (cast `BasePlayerCharacter` OtherActor))
  (bind _output_get (set `self.As Base Player Character` _asbase_player_character))
  (set `/Game/Characters/My_GameInstanse.local_save` (`self.GetTransform` _output_get) _as_my_game_instanse)
  (set `/Game/Characters/My_GameInstanse.save_active?` true _as_my_game_instanse)
  (bind _asbp_controller (cast `/Game/Characters/BP_Controller` (`GameplayStatics.GetPlayerController` 0)))
  (`/Game/Characters/BP_Controller.Event_save` _asbp_controller))

(fn `UserConstructionScript`)