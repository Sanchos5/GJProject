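; Player controller for a fruit-character game, handling form switching, health, checkpoints and the UI.
; Keys 1–4 swap pawns by spawning, possessing and destroying the old one, with later fruits gated by unlock count.
; Events push health, unlocks and current fruit to the HUD and open pause, game-over and victory widgets.
; Restart restores saved HP and fruit (first three only) at the GameInstance checkpoint, or reloads the level without a save.
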(event `self.ReceiveBeginPlay`
  ;[1 0 0] BeginPlay тут
  (`GameplayStatics.PlaySound2D` "/Game/Sound/s_play.s_play" 1.0 1.0 0.0 null null)
  (`WidgetBlueprintLibrary.SetInputMode_GameOnly` self)
  (bind _asmy_game_instanse (cast `/Game/Characters/My_GameInstanse` (`GameplayStatics.GetGameInstance`)))
  (set `self.As My Game Instanse` _asmy_game_instanse)
  (`self.Event_interfase`)
  (`self.Event_skolko_fructov_start`)
  (`self.Event_vid_frukta`)
  (bind _asbp_orange (cast `/Game/Characters/BP_Orange` (`GameplayStatics.GetPlayerPawn` 0)))
  (set `self.Target` _asbp_orange))

(event `Event_1`
  (`self.ChangePawn` (`self.bp_pineapple`) :!label _label)
  ;[1 1 1] Изменение иконок
  (set `self.i_vid_frukta` 1)
  (`self.Event_vid_frukta` :!label _label_2))

(event `Key|One`
  (params (Key :type "Key Structure"))
  (:`Pressed`
    (goto _label)))

(event `InputAction|upr_test_p`
  (params (Key :type "Key Structure")))

(event `Event_2`
  (if (>= (`self.i_skolko_fruktov`) 2) :!label _label_3
    (`self.ChangePawn` (`self.BP_cherry`))
    ;[1 1 1] Изменение иконок
    (set `self.i_vid_frukta` 2)
    (goto _label_2)))

(event `Key|Two`
  (params (Key :type "Key Structure"))
  (:`Pressed`
    (goto _label_3)))

(event `InputAction|upr_esc`
  (params (Key :type "Key Structure"))
  ;[1 1 1] Пауза
  (:`Pressed`
    (bind _returnvalue (`|CreateWidget` "/Game/Widget/WBP_pause.WBP_pause_C"))
    (`UserWidget.AddToViewport` _returnvalue 0)
    (set `/Game/Widget/WBP_pause.bp_controller` self _returnvalue)))

(event `Event_3`
  (if (>= (`self.i_skolko_fruktov`) 3) :!label _label_4
    (`self.ChangePawn` (`self.bp_orange`))
    ;[1 1 1] Изменение иконок
    (set `self.i_vid_frukta` 3)
    (goto _label_2)))

(event `Key|Three`
  (params (Key :type "Key Structure"))
  (:`Pressed`
    (goto _label_4)))

(event `Event_interfase`
  ;[1 1 1] Выведи интерфейс
  (bind _returnvalue (`|CreateWidget` "/Game/Widget/WBP_interface.WBP_interface_C"))
  (bind _output_get (set `self.WBP` _returnvalue))
  (`UserWidget.AddToViewport` _output_get 0))

(event `Event_4`
  (if (>= (`self.i_skolko_fruktov`) 4) :!label _label_5
    (`self.ChangePawn` (`self.bp_dragon`))
    ;[1 1 1] Изменение иконок
    (set `self.i_vid_frukta` 4)
    (goto _label_2)))

(event `Event_Damage`
  ;[1 1 1] Событие для дамага
  (bind _output_get (set `self.HP` (- (`self.HP`) 1)))
  (if (> _output_get 0)
    (`/Game/Widget/WBP_interface.Event_Heart` (`self.WBP`))
    (`GameplayStatics.PlaySound2D` "/Game/Sound/S_DamageTaken.S_DamageTaken" 1.0 1.0 0.0 null null)
    (else
      ;[1 1 1] Если хп кончилось, то выведи сообщение об этом
      (bind _returnvalue (`|CreateWidget` "/Game/Widget/WBP_GameOver.WBP_GameOver_C"))
      (`UserWidget.AddToViewport` _returnvalue 0)
      (set `/Game/Widget/WBP_GameOver.bp_controller` self _returnvalue)
      (`GameplayStatics.PlaySound2D` "/Game/Sound/S_DeathBackground.S_DeathBackground" 1.0 1.0 0.0 null null))))

(event `Key|Four`
  (params (Key :type "Key Structure"))
  (:`Pressed`
    (goto _label_5)))

(event `Event_save`
  ;[1 1 1] Сохранение данных при сейве
  (set `self.HP_save` (`self.HP`))
  (set `self.vid_frukta_save` (`self.i_vid_frukta`)))

(event `Event_skolko_fructov`
  (bind _wbp (`self.WBP`))
  ;[1 1 1] Вызови этот эвент при изменении числа разблокированных фруктов
  (`GameplayStatics.PlaySound2D` "/Game/Sound/S_NewCharacterUnlocked1.S_NewCharacterUnlocked1" 1.0 1.0 0.0 null null)
  (set `/Game/Widget/WBP_interface.i_skolko_fruktov` (`self.i_skolko_fruktov`) _wbp :!label _label_6)
  (`/Game/Widget/WBP_interface.Event_skolko_fruktov?` _wbp))

(event `Event_skolko_fructov_start`
  (goto _label_6))

(event `Event_restart`
  (bind (_local_save_location _local_save_rotation) (`KismetMathLibrary.BreakTransform` (`/Game/Characters/My_GameInstanse.local_save` (`self.As My Game Instanse`))))
  (if (`/Game/Characters/My_GameInstanse.save_active?` (`self.As My Game Instanse`))
    ;[1 1 1] Поставь такие характеристики, которые были при сейве и перезапусти интерфейс
    (`Widget.RemoveFromParent` (`self.WBP`))
    (set `self.HP` (`self.HP_save`))
    (`self.Event_interfase`)
    (`/Game/Widget/WBP_interface.Event_Heart` (`self.WBP`))
    (switch `int` (`self.vid_frukta_save`)
      (:`1`
        (`self.Event_1`))
      (:`2`
        (`self.Event_2`))
      (:`3`
        (`self.Event_3`)))
    ;[1 1 1] Если игрок посетил чекпоинт, то перемести его туда
    (set `self.bShowMouseCursor` false)
    (`self.K2_TeleportTo` (`GameplayStatics.GetPlayerPawn` 0) _local_save_location _local_save_rotation)
    (else
      ;[1 1 1] Если игрок ни разу не сохранился - перезапусти уровень
      (bind _returnvalue (`GameplayStatics.GetCurrentLevelName` true))
      (`GameplayStatics.OpenLevel` (`KismetStringLibrary.Conv_StringToName` _returnvalue)))))

(event `Event_vid_frukta`
  (bind _wbp (`self.WBP`))
  ;[1 1 1] Если персонаж меняет вид, надо вызвать этот эвент для обновления иконок
  (set `/Game/Widget/WBP_interface.i_vid_frukta` (`self.i_vid_frukta`) _wbp)
  (`/Game/Widget/WBP_interface.Event_vid_frukta` _wbp))

(event `Event_victory`
  (bind _returnvalue (`|CreateWidget` "/Game/Widget/WBP_Victory.WBP_Victory_C"))
  (`UserWidget.AddToViewport` _returnvalue 0))

(fn `ChangePawn`
  (params (PawnClasstoPossess :type "BasePlayerCharacter Class Reference"))
  (locals (OldPawn :type "Character Object Reference"))
  (bind _returnvalue (`GameplayStatics.GetPlayerCharacter` 0))
  (bind _oldpawn (`local.OldPawn`))
  (if (!= (`GameplayStatics.GetObjectClass` _returnvalue) PawnClasstoPossess)
    (set `local.OldPawn` _returnvalue)
    (bind _returnvalue_2 (`|SpawnActorFromClass` PawnClasstoPossess (`self.GetTransform` _returnvalue) "AlwaysSpawn" "MultiplyWithRoot" null null))
    (`self.Possess` _returnvalue_2)
    (`/Engine/EditorBlueprintResources/StandardMacros.IsValid` _oldpawn
      (:`Is Valid`
        (`self.K2_DestroyActor` _oldpawn)))))

(fn `UserConstructionScript`)