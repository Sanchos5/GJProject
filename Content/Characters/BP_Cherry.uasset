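; BP_Cherry is a cherry fruit character that collects other fruit and can transfer control to a travel cannon.
; Pressing E sphere-checks for a nearby BP_CannonToTravel, possesses it, shows its path, hides its widget and destroys the cherry.
; Capsule overlap with a non-player cherry, dragon fruit or orange sets a type-specific ISkolkoFruktov value on BP_Controller, fires EventSkolkoFructov and destroys that fruit.
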(event `Key|E`
  (params (Key :type "Key Structure"))
  (:`Pressed`
    (bind _outactors (`KismetSystemLibrary.SphereOverlapActors` (`self.K2_GetActorLocation`) 50.0 (`|MakeArray` "ObjectTypeQuery1" "ObjectTypeQuery2" "ObjectTypeQuery3" :!type "EObjectTypeQuery Enum") "/Game/Cannon/BP_CannonToTravel.BP_CannonToTravel_C" (`|MakeArray` self :!type "Actor Object Reference")))
    (for _index (range (`KismetArrayLibrary.Array_Length` _outactors))
      (bind _asbp_cannon_to_travel (cast `/Game/Cannon/BP_CannonToTravel` (`|GetArrayItem` _outactors _index)))
      (`Controller.Possess` (`GameplayStatics.GetPlayerController` 0) _asbp_cannon_to_travel)
      (`/Game/Cannon/BP_CannonToTravel.Show Path` _asbp_cannon_to_travel)
      (`/Game/Cannon/BP_CannonToTravel.Hide Widget` _asbp_cannon_to_travel)
      (`self.K2_DestroyActor`))))

(event `self.CapsuleComponent.OnComponentBeginOverlap`
  (params (OverlappedComponent :type "PrimitiveComponent Object Reference") (OtherActor :type "Actor Object Reference") (OtherComp :type "PrimitiveComponent Object Reference") (OtherBodyIndex :type Integer) (bFromSweep :type Boolean) (SweepResult :type "HitResult Structure (by ref)"))
  (bind _asbp_cherry (cast `/Game/Characters/BP_Cherry` OtherActor)
    (:`then`
      (if (not (`/Game/Characters/BP_Cherry.player?` _asbp_cherry))
        (bind _asbp_controller (cast `/Game/Characters/BP_Controller` (`GameplayStatics.GetPlayerController` 0)))
        (set `/Game/Characters/BP_Controller.i_skolko_fruktov` 2 _asbp_controller)
        (`/Game/Characters/BP_Controller.Event_skolko_fructov` _asbp_controller)
        (`self.K2_DestroyActor` OtherActor :!label _label)))
    (:`CastFailed`
      (bind _asbp_dragon_fruit (cast `/Game/Characters/BP_DragonFruit` OtherActor)
        (:`then`
          (if (not (`/Game/Characters/BP_DragonFruit.player?` _asbp_dragon_fruit))
            (bind _asbp_controller_2 (cast `/Game/Characters/BP_Controller` (`GameplayStatics.GetPlayerController` 0)))
            (set `/Game/Characters/BP_Controller.i_skolko_fruktov` 4 _asbp_controller_2)
            (`/Game/Characters/BP_Controller.Event_skolko_fructov` _asbp_controller_2)
            (goto _label)))
        (:`CastFailed`
          (bind _asbp_orange (cast `/Game/Characters/BP_Orange` OtherActor))
          (if (not (`/Game/Characters/BP_Orange.player?` _asbp_orange))
            (bind _asbp_controller_3 (cast `/Game/Characters/BP_Controller` (`GameplayStatics.GetPlayerController` 0)))
            (set `/Game/Characters/BP_Controller.i_skolko_fruktov` 3 _asbp_controller_3)
            (`/Game/Characters/BP_Controller.Event_skolko_fructov` _asbp_controller_3)
            (goto _label)))))))

(fn `UserConstructionScript`)