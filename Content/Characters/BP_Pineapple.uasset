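; BP_Pineapple is a fruit character that slows time and absorbs other fruits on touch.
; Holding the upr_shift input lowers global time dilation while raising its own CustomTimeDilation, so it moves faster than the world.
; Capsule overlap casts for Cherry, DragonFruit or Orange, sets BP_Controller's fruit count per type, fires its update event and destroys the fruit.
; Cherry and Orange are skipped when their Player flag is set, while DragonFruit is always taken.
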(event `InputAction|upr_shift`
  (params (Key :type "Key Structure"))
  ;[1 1 1] Механика замедления времени
  (:`Pressed`
    (`GameplayStatics.SetGlobalTimeDilation` 0.1)
    (set `self.CustomTimeDilation` 5.0))
  (:`Released`
    (`GameplayStatics.SetGlobalTimeDilation` 1.0)
    (set `self.CustomTimeDilation` 1.0)))

(event `self.CapsuleComponent.OnComponentBeginOverlap`
  (params (OverlappedComponent :type "PrimitiveComponent Object Reference") (OtherActor :type "Actor Object Reference") (OtherComp :type "PrimitiveComponent Object Reference") (OtherBodyIndex :type Integer) (bFromSweep :type Boolean) (SweepResult :type "HitResult Structure (by ref)"))
  (bind _asbp_cherry (cast `/Game/Characters/BP_Cherry` OtherActor)
    (:`then`
      (if (not (`/Game/Characters/BP_Cherry.player?` _asbp_cherry))
        (bind _asbp_controller (cast `/Game/Characters/BP_Controller` (`GameplayStatics.GetPlayerController` 0)))
        (set `/Game/Characters/BP_Controller.i_skolko_fruktov` 2 _asbp_controller)
        (`/Game/Characters/BP_Controller.Event_skolko_fructov` _asbp_controller)
        (`self.K2_DestroyActor` OtherActor :!label _label)))
    (:`CastFailed`
      (cast `/Game/Characters/BP_DragonFruit` OtherActor
        (:`then`
          (if true
            (bind _asbp_controller_2 (cast `/Game/Characters/BP_Controller` (`GameplayStatics.GetPlayerController` 0)))
            (set `/Game/Characters/BP_Controller.i_skolko_fruktov` 3 _asbp_controller_2)
            (`/Game/Characters/BP_Controller.Event_skolko_fructov` _asbp_controller_2)
            (goto _label)))
        (:`CastFailed`
          (bind _asbp_orange (cast `/Game/Characters/BP_Orange` OtherActor))
          (if (not (`/Game/Characters/BP_Orange.player?` _asbp_orange))
            (bind _asbp_controller_3 (cast `/Game/Characters/BP_Controller` (`GameplayStatics.GetPlayerController` 0)))
            (set `/Game/Characters/BP_Controller.i_skolko_fruktov` 4 _asbp_controller_3)
            (`/Game/Characters/BP_Controller.Event_skolko_fructov` _asbp_controller_3)
            (goto _label)))))))

(fn `UserConstructionScript`)