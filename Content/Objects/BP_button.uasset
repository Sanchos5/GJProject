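; BP_button is a one-shot button that switches off a linked damage-zone trap.
; A hit on its Cube by the player character or a BP_ProjectileToTravel, while Active, halves the cube's Z scale and deactivates both BpDamageZone and the button.
; Without a valid trap reference it prints a Russian warning and stays Active, so each further hit squashes the cube again.
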(event `self.Cube.OnComponentHit`
  (params (HitComponent :type "PrimitiveComponent Object Reference") (OtherActor :type "Actor Object Reference") (OtherComp :type "PrimitiveComponent Object Reference") (NormalImpulse :type "Vector Structure") (Hit :type "HitResult Structure (by ref)"))
  (bind _cube (`self.Cube`))
  (bind _bp_damage_zone (`self.bp_damage_zone`))
  (bind (_relativescale3d_x _relativescale3d_y _relativescale3d_z) (`KismetMathLibrary.BreakVector` (`SceneComponent.RelativeScale3D` _cube)))
  (cast `BasePlayerCharacter` OtherActor
    (:`then`
      _)
    (:`CastFailed`
      (cast `/Game/Cannon/BP_ProjectileToTravel` OtherActor)))
  (if (`self.active`)
    (`SceneComponent.SetRelativeScale3D` _cube (`KismetMathLibrary.MakeVector` _relativescale3d_x _relativescale3d_y (/ _relativescale3d_z 2.0)))
    (`/Engine/EditorBlueprintResources/StandardMacros.IsValid` _bp_damage_zone
      (:`Is Valid`
        (set `/Game/Objects/BP_damage_zone.active` false _bp_damage_zone)
        (set `self.active` false))
      (:`Is Not Valid`
        (`KismetSystemLibrary.PrintString` "Укажи в кнопке ссылку на ловушку")))))

(fn `UserConstructionScript`)