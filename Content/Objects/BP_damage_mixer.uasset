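; BP_damage_mixer is a spinning hazard that damages the player on contact.
; Tick spins the actor around yaw at the Skorost rate, while a separate timeline rotation event, not triggered from BeginPlay, turns yaw or pitch based on Horizontalvertical.
; Hits on either static mesh by a BasePlayerCharacter call EventDamage on the first player's BP_Controller, with the Active flag and a short delay throttling repeat damage.
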(event `self.ReceiveTick`
  (params (DeltaSeconds :type "Float (single-precision)"))
  (`self.K2_AddActorLocalRotation` (`KismetMathLibrary.MakeRotator` 0.0 0.0 (* (`GameplayStatics.GetWorldDeltaSeconds`) (`self.skorost`)))))

(event `Event_rotation`
  (bind (_start_rotation_roll _start_rotation_pitch _start_rotation_yaw) (`KismetMathLibrary.BreakRotator` (`self.start rotation`)))
  (bind (_start_rotation_roll_2 _start_rotation_pitch_2 _start_rotation_yaw_2) (`KismetMathLibrary.BreakRotator` (`self.start rotation`)))
  (if (`self.horizontal-vertical`)
    (set `self.start rotation` (`self.K2_GetActorRotation`))
    (bind (_direction _newtrack_0) (`Timeline|Timeline` :!via `PlayFromStart`)
      (:`Update`
        (bind _output_get (set `self.new_rotation` (`KismetMathLibrary.MakeRotator` _start_rotation_roll_2 _start_rotation_pitch_2 (+ _start_rotation_yaw_2 (* _newtrack_0 (`self.skorost`))))))
        (`self.K2_SetActorRotation` _output_get))
      (:`Finished`
        (`self.Event_rotation`)))
    (else
      (set `self.start rotation` (`self.K2_GetActorRotation`))
      (bind (_direction_2 _newtrack_0_2) (`Timeline|Timeline_0` :!via `PlayFromStart`)
        (:`Update`
          (bind _output_get_2 (set `self.new_rotation` (`KismetMathLibrary.MakeRotator` _start_rotation_roll (+ _start_rotation_pitch (* _newtrack_0_2 (`self.skorost`))) _start_rotation_yaw)))
          (`self.K2_SetActorRotation` _output_get_2))
        (:`Finished`
          (`self.Event_rotation`))))))

(event `self.ReceiveBeginPlay`)

(event `self.StaticMesh1.OnComponentHit`
  (params (HitComponent :type "PrimitiveComponent Object Reference") (OtherActor :type "Actor Object Reference") (OtherComp :type "PrimitiveComponent Object Reference") (NormalImpulse :type "Vector Structure") (Hit :type "HitResult Structure (by ref)"))
  (cast `BasePlayerCharacter` OtherActor)
  (if (`self.active`) :!label _label
    (bind _asbp_controller (cast `/Game/Characters/BP_Controller` (`GameplayStatics.GetPlayerController` 0)))
    (`/Game/Characters/BP_Controller.Event_Damage` _asbp_controller)
    (set `self.active` false)
    (`KismetSystemLibrary.Delay` 0.5)
    (set `self.active` true)))

(event `self.StaticMesh.OnComponentHit`
  (params (HitComponent :type "PrimitiveComponent Object Reference") (OtherActor :type "Actor Object Reference") (OtherComp :type "PrimitiveComponent Object Reference") (NormalImpulse :type "Vector Structure") (Hit :type "HitResult Structure (by ref)"))
  (cast `BasePlayerCharacter` OtherActor)
  (goto _label))

(fn `UserConstructionScript`)