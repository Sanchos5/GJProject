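; Damage zone that hurts the player when a BasePlayerCharacter starts overlapping its Cube component.
; While the Active flag is set, the overlap calls EventDamage on BP_Controller, always taken from player index 0.
; The Zaderzka flag gives a half-second cooldown between hits.
; Damage fires only on overlap begin, so staying inside the cube does not repeat it.
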(event `self.Cube.OnComponentBeginOverlap`
  (params (OverlappedComponent :type "PrimitiveComponent Object Reference") (OtherActor :type "Actor Object Reference") (OtherComp :type "PrimitiveComponent Object Reference") (OtherBodyIndex :type Integer) (bFromSweep :type Boolean) (SweepResult :type "HitResult Structure (by ref)"))
  (cast `BasePlayerCharacter` OtherActor)
  (if (and (`self.zaderzka`) (`self.active`))
    (bind _asbp_controller (cast `/Game/Characters/BP_Controller` (`GameplayStatics.GetPlayerController` 0)))
    (`/Game/Characters/BP_Controller.Event_Damage` _asbp_controller)
    (set `self.zaderzka` false)
    (`KismetSystemLibrary.Delay` 0.5)
    (set `self.zaderzka` true)))

(fn `UserConstructionScript`)